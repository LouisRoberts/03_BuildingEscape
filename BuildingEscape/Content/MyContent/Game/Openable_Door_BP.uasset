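; Openable door actor that swings open and closed in response to OpenDoor open and close requests.
; On BeginPlay it stores its initial rotation, and a timeline adds an animated yaw angle to that base rotation each update.
; Closing reverses the same timeline, and a timeline event track plays a squeaky door sound at the actor's location.
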(event `self.ReceiveBeginPlay`
  (set `self.InitialRotation` (`self.K2_GetActorRotation`)))

(event `self.OpenDoor.OnOpenRequest`
  (bind (_direction _open_angle) (`Timeline|Timeline_0` :!label _label)
    (:`Update`
      (`self.K2_SetActorRotation` (`KismetMathLibrary.ComposeRotators` (`KismetMathLibrary.MakeRotator` 0.0 0.0 _open_angle) (`self.InitialRotation`))))
    (:`SoundTiming`
      (`GameplayStatics.PlaySoundAtLocation` "/Game/MyContent/Audio/squeaky_closet_door_open_001_16bit.squeaky_closet_door_open_001_16bit" (`self.K2_GetActorLocation`)))))

(event `self.OpenDoor.OnCloseRequest`
  (goto _label :!via `Reverse`))

(fn `UserConstructionScript`)